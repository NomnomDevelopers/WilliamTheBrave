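; HealthDroplets is a short-lived physics droplet that sends its Damage value to an overlapping actor through a CanTakeDamage message, then destroys itself.
; A brief delay after BeginPlay opens a gate that lets Sphere1 overlaps trigger that message.
; Hitting an actor without the "BP" tag stops Sphere's physics and deactivates the particle system.
; Tick steadily shrinks Sphere and destroys the droplet once its scale drops below zero.
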(event OnComponentBeginOverlap(Sphere1)
  (params (OtherActor :type Actor%20Object%20Reference) (OtherComp :type Primitive%20Component%20Object%20Reference) (OtherBodyIndex :type Integer) (bFromSweep :type Boolean) (SweepResult :type Hit%20Result%20Structure%20%28by%20ref%29))
  (Utilities|FlowControl|Gate true
    (:Exit
      (Class|DamageInterface|CanTakeDamage(Message) OtherActor (Variables|Default|GetDamage) (Utilities|GetClassDisplayName (Utilities|GetClass self)) self)
      (Actor|DestroyActor))))

(event OnComponentHit(Sphere)
  (params (OtherActor :type Actor%20Object%20Reference) (OtherComp :type Primitive%20Component%20Object%20Reference) (NormalImpulse :type Vector :default "0, 0, 0") (Hit :type Hit%20Result%20Structure%20%28by%20ref%29))
  (if (not (Actor|ActorHasTag OtherActor "BP"))
    (Physics|SetSimulatePhysics false)
    (Components|Activation|Deactivate (Variables|Default|GetParticleSystem1))))

(event EventBeginPlay
  (Utilities|FlowControl|Delay 0.4)
  (Utilities|FlowControl|Sequence
    (:then_0
      (Utilities|FlowControl|Gate true) ; enters at Open
    )))

(event EventTick
  (params (DeltaSeconds :type Float%20%28single-precision%29))
  (bind _returnvalue (/ DeltaSeconds 155.0))
  (bind _sphere (Variables|Default|GetSphere))
  (bind _sphere_2 (Variables|Default|GetSphere))
  (bind _returnvalue_2 (Transformation|GetWorldScale _sphere_2))
  (bind _returnvalue_3 (Transformation|GetWorldScale _sphere))
  (Transformation|SetWorldScale3D (Variables|Default|GetSphere) (Math|Vector|MakeVector (- (.x _returnvalue_3) _returnvalue) (- (.y _returnvalue_3) _returnvalue) (- (.z _returnvalue_3) _returnvalue)))
  (if (Math|Boolean|ORBoolean (< (.x _returnvalue_2) 0.0) (< (.y _returnvalue_2) 0.0) (< (.z _returnvalue_2) 0.0))
    (Actor|DestroyActor)))

(fn ConstructionScript)