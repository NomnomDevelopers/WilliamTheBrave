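; SphereMob is a sentry enemy that plays red light, green light, shooting at fast-moving Playable actors inside its detection box.
; The box, offset ahead in the construction script, maintains a target array.
; A once-per-second throttled Tick turns toward the first target via timeline lerp, or resets rotation when none remain.
; Fast horizontal movement triggers a red light and charge, then a delayed Flameo spawn and return to green.
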(event OnComponentBeginOverlap(Box)
  (params (OtherActor :type Actor%20Object%20Reference) (OtherComp :type Primitive%20Component%20Object%20Reference) (OtherBodyIndex :type Integer) (bFromSweep :type Boolean) (SweepResult :type Hit%20Result%20Structure%20%28by%20ref%29))
  (bind _target (Variables|Default|GetTarget))
  ;[1 1 1] Add targets to target array
  (if (Actor|ActorHasTag OtherActor "Playable")
    (Utilities|Array|Add _target OtherActor)
    (if (> (Utilities|Array|Length _target) 0)
      _)))

(event OnComponentEndOverlap(Box)
  (params (OtherActor :type Actor%20Object%20Reference) (OtherComp :type Primitive%20Component%20Object%20Reference) (OtherBodyIndex :type Integer))
  (bind _target (Variables|Default|GetTarget))
  ;[1 1 1] Add targets to target array
  (if (Actor|ActorHasTag OtherActor "Playable")
    (Utilities|Array|RemoveItem _target OtherActor)
    (if (== (Utilities|Array|Length _target) 0)
      _)))

(event Custom|FirinMuhLazoe
  ;[1 1 1] Firing My Laser Event
  (Game|SpawnActorfromClass "/Game/Blueprints/Flameo.Flameo_C" (Math|Transform|MakeTransform (Transformation|GetWorldLocation (Variables|Default|GetLaserSpawn)) (Transformation|GetActorRotation self) "1,1,1") true 0))

(event Custom|LightGreen
  ;[1 1 1] Red Yellow Green
  (bind (_direction _0s0 _0s255) (Timeline|PointLightColorChanger Play)
    (:Update
      (Rendering|Components|Light|SetLightColor (Variables|Default|GetPointLight) (Utilities|Struct|MakeLinearColor _0s255 _0s0 0.0 1.0)))))

(event Custom|LightRed
  ;[1 1 1] Red Yellow Green
  (bind (_direction _0s0 _0s255) (Timeline|PointLightColorChanger Reverse)
    (:Update
      (Rendering|Components|Light|SetLightColor (Variables|Default|GetPointLight) (Utilities|Struct|MakeLinearColor _0s255 _0s0 0.0 1.0)))))

(event EventTick
  (params (DeltaSeconds :type Float%20%28single-precision%29))
  (bind _target (Variables|Default|GetTarget))
  (bind _item (Utilities|Array|Get(acopy) _target))
  (bind _returnvalue (Transformation|GetVelocity _item))
  ;[1 1 1] Tick Limiter, choose an action once a second
  (bind _output_get (Variables|Default|SetTickLimiterCounter (+ DeltaSeconds (Variables|Default|GetTickLimiterCounter))))
  (if (> _output_get 1.0)
    (Variables|Default|SetTickLimiterCounter 0.0)
    ;[1 1 1] If theres a target
    (if (> (Utilities|Array|Length (Variables|Default|GetTarget)) 0)
      ;[1 1 1] If Sphere is readying to shoot
      (if (Variables|Default|GetChargin)
        ;[1 1 1] Chargin!
        (Utilities|FlowControl|Delay 2.0)
        (CallFunction|FirinMuhLazoe)
        (Variables|Default|SetChargin false)
        (CallFunction|LightGreen)
        (else
          ;[1 1 1] Look at the target
          (bind _output_get_2 (Variables|Default|SetLookRotationBeforeLerp (Transformation|GetActorRotation self)))
          (bind _0_to_1 (Timeline|Timeline_0 PlayFromStart)
            (:Update
              (Transformation|SetActorRotation self (Math|Rotator|Lerp(Rotator) _output_get_2 (Math|Rotator|FindLookatRotation (Transformation|GetActorLocation) (Transformation|GetActorLocation (Utilities|Array|Get(acopy) (Variables|Default|GetTarget)))) _0_to_1)))
            (:Finished
              ;[1 1 1] Fire upon fast moving objects
              (if (> (+ (Math|Float|Absolute(Float) (.x _returnvalue)) (Math|Float|Absolute(Float) (.y _returnvalue))) 5.7e+02)
                (Variables|Default|SetChargin true)
                (CallFunction|LightRed))))))
      (else
        (Transformation|SetActorRotation "0, 0, 0")))))

(fn ConstructionScript
  (bind _self self)
  (bind _returnvalue (Transformation|GetActorRotation _self))
  (Utilities|FlowControl|DoOnce false
    (:Completed
      (Transformation|SetWorldLocationAndRotation (Variables|Default|GetBox) (+ (Transformation|GetActorLocation _self) (Math|Vector|RotateVector (Math|Vector|MakeVector 3808.0 0.0 0.0) _returnvalue)) _returnvalue false))))