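; CloseEnough is a behavior tree decorator that gates AI behavior on the distance between the controlled pawn and its follow target.
; It casts the owner to AI_Con, caches it, and reads the TargetToFollow actor from the blackboard.
; Despite the name, the condition passes when the straight-line distance is at least AcceptableDistance, meaning the pawn is not yet close enough.
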(fn PerformConditionCheck
  (params (OwnerActor :type Actor%20Object%20Reference))
  (bind _asai_con (Utilities|Casting|CastToAI_Con OwnerActor))
  (Variables|Default|SetAI_CON_C _asai_con)
  (return (>= (Math|Vector|VectorLength (- (Transformation|GetActorLocation (AI|BehaviorTree|GetBlackboardValueasActor (Variables|Default|GetTargetToFollow))) (Transformation|GetActorLocation (Pawn|GetControlledPawn (Variables|Default|GetAI_CON_C))))) (Variables|Default|GetAcceptableDistance))))