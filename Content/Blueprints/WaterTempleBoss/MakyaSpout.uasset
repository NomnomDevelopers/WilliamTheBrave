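; Water spout hazard for the Makya water temple boss that damages and lifts whatever stands inside it.
; Static mesh overlaps maintain an actor list, and every tick each listed actor receives a damage message.
; Characters also get a small additive upward launch, with vertical speed capped by an override.
; The construction script traces vertically over a scale-adjusted span and snaps the actor's height to the hit surface.
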(event OnComponentBeginOverlap(StaticMesh)
  (params (OtherActor :type Actor%20Object%20Reference) (OtherComp :type Primitive%20Component%20Object%20Reference) (OtherBodyIndex :type Integer) (bFromSweep :type Boolean) (SweepResult :type Hit%20Result%20Structure%20%28by%20ref%29))
  (Utilities|Array|AddUnique (Variables|Default|GetActorArray) OtherActor))

(event OnComponentEndOverlap(StaticMesh)
  (params (OtherActor :type Actor%20Object%20Reference) (OtherComp :type Primitive%20Component%20Object%20Reference) (OtherBodyIndex :type Integer))
  (Utilities|Array|RemoveItem (Variables|Default|GetActorArray) OtherActor))

(event EventTick
  (params (DeltaSeconds :type Float%20%28single-precision%29))
  (for _array_element (Variables|Default|GetActorArray)
    (Utilities|IsValid _array_element
      (:Is%20Valid
        (Class|DamageInterface|CanTakeDamage(Message) _array_element 1.0 (Utilities|GetClassDisplayName (Utilities|GetClass self)) self)
        (bind _ascharacter (Utilities|Casting|CastToCharacter _array_element))
        (if (<= (.z (Transformation|GetVelocity _ascharacter)) 1.5e+03)
          (Character|LaunchCharacter _ascharacter "0, 0,40.000000" false false)
          (else
            (Character|LaunchCharacter _ascharacter (Math|Vector|MakeVector 0.0 0.0 1501.0) false true)))))))

(fn ConstructionScript
  (bind _returnvalue (Transformation|GetActorLocation))
  (bind _returnvalue_2 (Transformation|GetActorLocation))
  (bind _outhit (Collision|LineTraceForObjects (Math|Vector|MakeVector (.x _returnvalue_2) (.y _returnvalue_2) (+ (.z _returnvalue_2) (* (.z (Transformation|GetWorldScale)) (Math|Float|MakeLiteralFloat 678.0)))) (+ (Transformation|GetActorLocation) (Math|Vector|MakeVector 0.0 0.0 (* (.z (Transformation|GetWorldScale)) (Math|Float|MakeLiteralFloat 678.0) -1.0))) (Utilities|Array|MakeArray "ObjectTypeQuery1" "ObjectTypeQuery2") false 0 "ForOneFrame"))
  (Transformation|SetActorLocation (Math|Vector|MakeVector (.x _returnvalue) (.y _returnvalue) (.z (.location _outhit))) false))