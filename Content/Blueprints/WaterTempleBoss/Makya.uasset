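; Makya is a manually controlled water temple boss character with movement, look, jump and three water attacks on number keys.
; Splash fires a burst of MakyaSplash projectiles from a ground-traced point ahead, while Rain spawns MakyaRain at a random offset high overhead.
; Holding Expunge spawns splashes every Tick and re-steers all tracked ones using remapped look-at yaw from Makya, then releases them on key-up.
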(event Custom|SpawnMakyaSplash
  (bind _outhit_location (CallFunction|LineTraceforWorldStatic100UnitsAheadStraightDown))
  (for _index (range 0 40)
    (Game|SpawnActorfromClass "/Game/Blueprints/WaterTempleBoss/MakyaSplash.MakyaSplash_C" (Math|Transform|MakeTransform _outhit_location (Utilities|RotOfRandVectorinCone 45.0 15.0) "1,1,1") true 1.45e+03 0)))

(event Custom|SpawnMakyaRain
  (bind _returnvalue (Math|Trig|DegreesToRadians 45.0))
  (bind _returnvalue_2 (Class|KismetMathLibrary|RandomUnitVectorinCone "0, 0,1.000000" _returnvalue))
  (Game|SpawnActorfromClass "/Game/Blueprints/WaterTempleBoss/MakyaRain.MakyaRain_C" (Math|Transform|MakeTransform (+ (.location (Transformation|GetWorldTransform (Variables|Default|GetCylinder))) "0, 0,2000.000000" (Math|Vector|MakeVector (* (.x _returnvalue_2) 1.5e+03) (* (.y _returnvalue_2) 1.5e+03) 0.0)) "0, 0, 0" "1,1,1") true 0))

(event Custom|ChargeExpenge
  (bind _outhit_location (CallFunction|LineTraceforWorldStatic100UnitsAheadStraightDown))
  (for _index (range 0 15)
    (bind _returnvalue (Game|SpawnActorfromClass "/Game/Blueprints/WaterTempleBoss/MakyaSplash.MakyaSplash_C" (Math|Transform|MakeTransform _outhit_location (Utilities|RotOfRandVectorinCone 45.0 15.0) "1,1,1") true 2.6e+03 0))
    (Utilities|Array|Add (Variables|Default|GetExpungeArray) _returnvalue))
  (for _array_element (Variables|Default|GetExpungeArray)
    (Utilities|IsValid _array_element
      (:Is%20Valid
        (Game|Components|ProjectileMovement|SetVelocityinLocalSpace _array_element (Math|Vector|MakeVector (.x (* (Math|Vector|RotateVector (Math|Vector|MakeVector 0.0 1.0 0.0) (Math|Rotator|MakeRotator (.pitch (Math|Rotator|FindLookatRotation (Transformation|GetActorLocation) (Transformation|GetActorLocation _array_element))) (Class|KismetMathLibrary|MapRange (.yaw (Math|Rotator|FindLookatRotation (Transformation|GetActorLocation) (Transformation|GetActorLocation _array_element))) -1.8e+02 1.8e+02 0.0 7.2e+02) (.roll (Math|Rotator|FindLookatRotation (Transformation|GetActorLocation) (Transformation|GetActorLocation _array_element))))) 1.45e+03)) (.y (* (Math|Vector|RotateVector (Math|Vector|MakeVector 0.0 1.0 0.0) (Math|Rotator|MakeRotator (.pitch (Math|Rotator|FindLookatRotation (Transformation|GetActorLocation) (Transformation|GetActorLocation _array_element))) (Class|KismetMathLibrary|MapRange (.yaw (Math|Rotator|FindLookatRotation (Transformation|GetActorLocation) (Transformation|GetActorLocation _array_element))) -1.8e+02 1.8e+02 0.0 7.2e+02) (.roll (Math|Rotator|FindLookatRotation (Transformation|GetActorLocation) (Transformation|GetActorLocation _array_element))))) 1.45e+03)) 1.1e+02))))))

(event EventTick
  (params (DeltaSeconds :type Float%20%28single-precision%29))
  (Utilities|FlowControl|Sequence
    (:then_0
      (if (Variables|Default|GetChargeExpunge)
        (CallFunction|ChargeExpenge)))))

(event Input|ActionEvents|InputActionJump
  ;[1 1 1] Manual movement
  (:Pressed
    (Character|Jump)))

(event Input|AxisEvents|InputAxisMouseLeft
  (params (AxisValue :type Float%20%28single-precision%29))
  ;[1 1 1] Manual movement
  (Pawn|Input|AddControllerYawInput AxisValue))

(event Input|AxisEvents|InputAxisMouseUp
  (params (AxisValue :type Float%20%28single-precision%29))
  ;[1 1 1] Manual movement
  (Pawn|Input|AddControllerPitchInput AxisValue))

(event Input|AxisEvents|InputAxisFoward
  (params (AxisValue :type Float%20%28single-precision%29))
  ;[1 1 1] Manual movement
  (Pawn|Input|AddMovementInput (Math|Vector|GetForwardVector (Class|KismetMathLibrary|MakeRot 0.0 (.yaw (Transformation|GetWorldRotation (Variables|Character|GetMesh))) 0.0)) AxisValue false))

(event Input|AxisEvents|InputAxisRight
  (params (AxisValue :type Float%20%28single-precision%29))
  ;[1 1 1] Manual movement
  (Pawn|Input|AddMovementInput (Math|Vector|GetRightVector (Class|KismetMathLibrary|MakeRot 0.0 (.yaw (Transformation|GetWorldRotation (Variables|Character|GetMesh))) 0.0)) AxisValue false))

(event Input|KeyboardEvents|1
  (:Pressed
    (CallFunction|SpawnMakyaSplash)))

(event Input|KeyboardEvents|2
  (:Pressed
    (CallFunction|SpawnMakyaRain)))

(event Input|KeyboardEvents|3
  (:Pressed
    (Variables|Default|SetChargeExpunge true))
  (:Released
    (Variables|Default|SetChargeExpunge false)
    (Utilities|Array|Clear (Variables|Default|GetExpungeArray))))

(event Input|KeyboardEvents|4)

(fn ConstructionScript)

(fn LineTraceforWorldStatic100UnitsAheadStraightDown
  (bind _outhit (Collision|LineTraceForObjects (+ (Math|Vector|RotateVector (Math|Vector|MakeVector 1e+02 0.0 0.0) (Math|Rotator|MakeRotator 0.0 (.yaw (Pawn|GetControlRotation :!class /Script/Engine.Pawn)) 0.0)) (Transformation|GetWorldLocation (Variables|Default|GetCylinder))) (+ (Math|Vector|RotateVector (Math|Vector|MakeVector 1e+02 0.0 -8e+02) (Math|Rotator|MakeRotator 0.0 (.yaw (Pawn|GetControlRotation :!class /Script/Engine.Pawn)) 0.0)) (Transformation|GetWorldLocation (Variables|Default|GetCylinder))) (Utilities|Array|MakeArray "ObjectTypeQuery1") false 0 "None"))
  (return (Math|Vector|MakeVector (.x (.location _outhit)) (.y (.location _outhit)) (+ (.z (.location _outhit)) 1e+02))))