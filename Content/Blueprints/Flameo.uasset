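; Flameo is a projectile that deals damage on its first bounce, then bursts into a spray of droplets and destroys itself.
; The bounce sends the hit actor a damage message, then spawns a random number of HealthDropletsv2 actors at random speeds, using a cone direction based on the impact normal.
; Overlapping a Makya Splash actor destroys the projectile without damage or droplets.
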(event OnComponentBeginOverlap(Sphere)
  (params (OtherActor :type Actor%20Object%20Reference) (OtherComp :type Primitive%20Component%20Object%20Reference) (OtherBodyIndex :type Integer) (bFromSweep :type Boolean) (SweepResult :type Hit%20Result%20Structure%20%28by%20ref%29))
  (switch string (Utilities|GetClassDisplayName (Utilities|GetClass OtherActor))
    (:MakyaSplash_C
      (Actor|DestroyActor))))

(event OnProjectileStop(ProjectileMovement)
  (params (ImpactResult :type Hit%20Result%20Structure%20%28by%20ref%29)))

(event OnProjectileBounce(ProjectileMovement)
  (params (ImpactResult :type Hit%20Result%20Structure%20%28by%20ref%29) (ImpactVelocity :type Vector%20%28by%20ref%29 :default "0, 0, 0"))
  (Utilities|FlowControl|DoOnce false
    (:Completed
      (Class|DamageInterface|CanTakeDamage(Message) (.hitactor ImpactResult) (Variables|Default|GetDamage) (Utilities|GetClassDisplayName (Utilities|GetClass self)) self)
      (Components|Movement|StopMovementImmediately)
      (bind _output_get (Variables|Default|SetRandVariable (Math|Random|RandomIntegerinRange 35 50)))
      (for _index (range 0 _output_get)
        (Game|SpawnActorfromClass "/Game/Blueprints/HealthDropletsv2.HealthDropletsv2_C" (Utilities|HealthDropletsv2 (.normal ImpactResult) 1.1e+02 0.6) true 5.0 (Math|Random|RandomFloatinRange 1.8e+03 2.5e+03) 0))
      (Actor|DestroyActor))))

(fn ConstructionScript)