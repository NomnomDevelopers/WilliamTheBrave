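; William is the player character Blueprint, with look and movement input, jumping, a grounded dash and lantern-fired flame projectiles.
; Health doubles as the resource: dashing, shooting and a debug launch-ball action each subtract from it.
; Shots spawn the current flame class ahead of the lantern through a DoOnce gate, reset after a per-class delay.
; CanTakeDamage switches on the source class, so Angry Camel hits apply knockback and resistance-reduced damage.
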(event Custom|ResetShootGate
  (bind _self self)
  (bind _returnvalue (Pawn|GetControlRotation _self :!class /Script/Engine.Pawn))
  ;[1 1 1] On shoot, decriment health, spawn a x, than x second delay before shooting again
  (Utilities|FlowControl|DoOnce false) ; enters at Reset
)

(event Custom|HitForDamage
  (params (Damage :type Float%20%28single-precision%29))
  ;[1 1 1] Taking Damage
  (bind _output_get (Variables|Default|SetHealth (- (Variables|Default|GetHealth) Damage)))
  (if (<= _output_get 0.0)
    (Development|PrintString "Gameoverlol")))

(event EventActorBeginOverlap
  (params (OtherActor :type Actor%20Object%20Reference)))

(event EventCanTakeDamage
  (params (DamageTaken :type Float%20%28single-precision%29) (FromWhat :type Object%20Class%20Reference) (FromWhom :type Actor%20Object%20Reference))
  (bind _returnvalue (Transformation|GetActorLocation FromWhom))
  (bind _returnvalue_2 (Transformation|GetActorLocation))
  (bind _returnvalue_3 (Class|KismetMathLibrary|GetDirectionVector _returnvalue _returnvalue_2))
  ;[1 1 1] Add things that deal damage here
  (switch string (Utilities|GetClassDisplayName FromWhat)
    (:Default
      (Development|PrintString "Event Not Described"))
    (:AngryCamel_C
      ;[1 1 1] Knockback when hit by angryCamel
      (Character|LaunchCharacter (Math|Vector|MakeVector (* (.x _returnvalue_3) 1.5e+03) (* (.y _returnvalue_3) 1.5e+03) (Class|CharacterMovementComponent|GetMaxJumpHeight (Variables|Character|GetCharacterMovement))) false false)
      (CallFunction|HitforDamage (* DamageTaken (- 1.0 (Variables|Default|GetPhysicalResist)))))))

(event Input|ActionEvents|InputActionJump
  ;[1 1 1] Basic movement
  (:Pressed
    (Character|Jump)))

(event Input|ActionEvents|InputActionShoot
  (bind _self self)
  (bind _returnvalue (Pawn|GetControlRotation _self :!class /Script/Engine.Pawn))
  ;[1 1 1] On shoot, decriment health, spawn a x, than x second delay before shooting again
  (:Pressed
    (Utilities|FlowControl|DoOnce false
      (:Completed
        (Variables|Default|SetHealth (- (Variables|Default|GetHealth) (Variables|Default|GetLeftClickCost)))
        (Game|SpawnActorfromClass (Variables|Default|GetCurrentFlameMode) (Math|Transform|MakeTransform (+ (Transformation|GetWorldLocation (Variables|Default|GetLantern)) (Math|Vector|RotateVector (Math|Vector|MakeVector 1e+02 0.0 0.0) (Math|Rotator|MakeRotator 0.0 (.yaw _returnvalue) 0.0))) (Math|Rotator|MakeRotator (.pitch _returnvalue) (.yaw _returnvalue) (.roll _returnvalue))) false 0)
        ;[1 1 1] Add flame mode fire delays here
        (switch string (Utilities|GetClassDisplayName (Variables|Default|GetCurrentFlameMode))
          (:Flameo_C
            (Utilities|FlowControl|Delay 1.0)
            (CallFunction|ResetShootGate)))))))

(event Input|ActionEvents|InputActionLauchyBall
  (bind _self self)
  (bind _returnvalue (Pawn|GetControlRotation _self :!class /Script/Engine.Pawn))
  ;[1 1 1] ToDo: Delete me
  (:Pressed
    (Game|SpawnActorfromClass "/Game/Blueprints/FlameoLaunchBall.FlameoLaunchBall_C" (Math|Transform|MakeTransform (+ (Transformation|GetWorldLocation (Variables|Default|GetLantern)) (Math|Vector|RotateVector (Math|Vector|MakeVector 1e+02 0.0 0.0) (Math|Rotator|MakeRotator 0.0 (.yaw _returnvalue) 0.0))) (Math|Rotator|MakeRotator (.pitch _returnvalue) (.yaw _returnvalue) (.roll _returnvalue))) false 0)
    (Variables|Default|SetHealth (- (Variables|Default|GetHealth) (Variables|Default|GetRightClickCost)))))

(event Input|ActionEvents|InputActionDash
  (bind _dashpower (Variables|Default|GetDashPower))
  ;[1 1 1] The character is moving AND is on the ground
  (:Pressed
    (if (and (not (AI|Components|NavMovement|IsFalling (Variables|Character|GetCharacterMovement))) (or (!= (stale Input|AxisEvents|InputAxisFoward AxisValue) 0.0) (!= (stale Input|AxisEvents|InputAxisRight AxisValue) 0.0)))
      ;[1 1 1] Decriment dash health cost
      (Variables|Default|SetHealth (- (Variables|Default|GetHealth) (Variables|Default|GetDashCost)))
      ;[1 1 1] Launch in the moving direction with the velocity of 1*dashpower*jumpheight
      (Character|LaunchCharacter (* (Math|Vector|RotateVector (Math|Vector|MakeVector (* (stale Input|AxisEvents|InputAxisFoward AxisValue) _dashpower) (* (stale Input|AxisEvents|InputAxisRight AxisValue) _dashpower) 1.0) (Math|Rotator|MakeRotator 0.0 (.yaw (Pawn|GetControlRotation self :!class /Script/Engine.Pawn)) 0.0)) (Class|CharacterMovementComponent|GetMaxJumpHeight (Variables|Character|GetCharacterMovement))) false false))))

(event Input|AxisEvents|InputAxisMouseLeft
  (params (AxisValue :type Float%20%28single-precision%29))
  ;[1 1 1] Basic movement
  (Pawn|Input|AddControllerYawInput AxisValue))

(event Input|AxisEvents|InputAxisMouseUp
  (params (AxisValue :type Float%20%28single-precision%29))
  ;[1 1 1] Basic movement
  (Pawn|Input|AddControllerPitchInput AxisValue))

(event Input|AxisEvents|InputAxisFoward
  (params (AxisValue :type Float%20%28single-precision%29))
  ;[1 1 1] Basic movement
  (Pawn|Input|AddMovementInput (Math|Vector|GetForwardVector (Class|KismetMathLibrary|MakeRot 0.0 (.yaw (Transformation|GetWorldRotation (Variables|Character|GetMesh))) 0.0)) AxisValue false))

(event Input|AxisEvents|InputAxisRight
  (params (AxisValue :type Float%20%28single-precision%29))
  ;[1 1 1] Basic movement
  (Pawn|Input|AddMovementInput (Math|Vector|GetRightVector (Class|KismetMathLibrary|MakeRot 0.0 (.yaw (Transformation|GetWorldRotation (Variables|Character|GetMesh))) 0.0)) AxisValue false))

(fn ConstructionScript)