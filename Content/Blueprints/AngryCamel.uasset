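; AngryCamel is a spinning, spiked enemy that chases Playable-tagged actors entering its sense range.
; A timeline winds up its rotation, and Tick moves it toward the first tracked target once spin nears full speed, winding down when none remain.
; Its spikes send damage to anything they overlap.
; Only Flameo C damage lowers its health; at zero it spawns a CubeofDeath DM actor and destroys itself.
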(event OnComponentBeginOverlap(SenseRange)
  (params (OtherActor :type Actor%20Object%20Reference) (OtherComp :type Primitive%20Component%20Object%20Reference) (OtherBodyIndex :type Integer) (bFromSweep :type Boolean) (SweepResult :type Hit%20Result%20Structure%20%28by%20ref%29))
  (bind _target (Variables|Default|GetTarget))
  ;[1 1 1] Enter and leave angering area
  (if (Actor|ActorHasTag OtherActor "Playable")
    (Utilities|Array|Add _target OtherActor)
    (if (> (Utilities|Array|Length _target) 0)
      (Variables|Default|SetActive true)
      (bind _yaw0to540 (Timeline|RotatingWindup Play)
        (:Update
          (Variables|/Script/Engine.RotatingMovementComponent|SetRotationRate (Variables|Default|GetRotatingMovement) (Math|Rotator|MakeRotator 0.0 _yaw0to540 0.0)))))))

(event OnComponentBeginOverlap(FrontAndBackSpikes)
  (params (OtherActor :type Actor%20Object%20Reference) (OtherComp :type Primitive%20Component%20Object%20Reference) (OtherBodyIndex :type Integer) (bFromSweep :type Boolean) (SweepResult :type Hit%20Result%20Structure%20%28by%20ref%29))
  ;[1 1 1] Hit stuff with spikes
  (Class|DamageInterface|CanTakeDamage(Message) OtherActor (Variables|Default|GetSpikeDamage) "" self))

(event OnComponentBeginOverlap(LeftAndRightSpikes)
  (params (OtherActor :type Actor%20Object%20Reference) (OtherComp :type Primitive%20Component%20Object%20Reference) (OtherBodyIndex :type Integer) (bFromSweep :type Boolean) (SweepResult :type Hit%20Result%20Structure%20%28by%20ref%29))
  ;[1 1 1] Hit stuff with spikes
  (Class|DamageInterface|CanTakeDamage(Message) OtherActor (Variables|Default|GetSpikeDamage) "" self))

(event OnComponentEndOverlap(SenseRange)
  (params (OtherActor :type Actor%20Object%20Reference) (OtherComp :type Primitive%20Component%20Object%20Reference) (OtherBodyIndex :type Integer))
  (bind _target (Variables|Default|GetTarget))
  ;[1 1 1] Enter and leave angering area
  (if (Actor|ActorHasTag OtherActor "Playable")
    (Utilities|Array|RemoveItem _target OtherActor)
    (if (== (Utilities|Array|Length _target) 0)
      (Variables|Default|SetActive false)
      (bind _yaw0to540 (Timeline|RotatingWindup Reverse)
        (:Update
          (Variables|/Script/Engine.RotatingMovementComponent|SetRotationRate (Variables|Default|GetRotatingMovement) (Math|Rotator|MakeRotator 0.0 _yaw0to540 0.0)))))))

(event Custom|HitForDamage
  (params (Damage :type Float%20%28single-precision%29 :default 0.0))
  ;[1 1 1] Taking damage
  (bind _output_get (Variables|Default|SetHealth (- (Variables|Default|GetHealth) Damage)))
  (if (<= _output_get 0.0)
    (CallFunction|Dying)))

(event Custom|Dying
  ;[1 1 1] Dying
  (Game|SpawnActorfromClass "/Game/Blueprints/CubeofDeathMesh_Cube_000_DM.CubeofDeathMesh_Cube_000_DM_C" (Transformation|GetActorTransform) true 0)
  (Actor|DestroyActor))

(event EventBeginPlay)

(event EventActorBeginOverlap
  (params (OtherActor :type Actor%20Object%20Reference)))

(event EventTick
  (params (DeltaSeconds :type Float%20%28single-precision%29))
  (if (Math|Boolean|ANDBoolean (Variables|Default|GetActive) (> (.yaw (Variables|/Script/Engine.RotatingMovementComponent|GetRotationRate (Variables|Default|GetRotatingMovement))) 4.5e+02) (> (Utilities|Array|Length (Variables|Default|GetTarget)) 0))
    (Pawn|Input|AddMovementInput (Class|KismetMathLibrary|GetDirectionVector (Transformation|GetActorLocation) (Transformation|GetActorLocation (Utilities|Array|Get(acopy) (Variables|Default|GetTarget)))) 1.0 false)))

(event EventCanTakeDamage
  (params (DamageTaken :type Float%20%28single-precision%29) (FromWhat :type String) (FromWhom :type Actor%20Object%20Reference))
  ;[1 1 1] List of things that can damage AngryCamel
  (switch string FromWhat
    (:Flameo_C
      (CallFunction|HitforDamage DamageTaken))))

(fn ConstructionScript)