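; Health droplet projectile that sends a damage-interface message to overlapping actors, apparently as a health pickup, then flags itself to auto-destroy.
; Gates hold both overlap spheres closed briefly after spawn: SphereCollision serves only William, while Sphere serves any actor except Makya Splash, which destroys it outright.
; The droplet keeps bouncing off "BP"-tagged actors but sticks to others, deactivating its particles on stop.
; Tick shrinks Sphere until auto-destroy is flagged.
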(event OnProjectileBounce(ProjectileMovement)
  (params (ImpactResult :type Hit%20Result%20Structure%20%28by%20ref%29) (ImpactVelocity :type Vector%20%28by%20ref%29 :default "0, 0, 0"))
  ;[1 0.008681 0] Bounce off certain actors, stick to everything else
  (if (not (Actor|ActorHasTag (.hitactor ImpactResult) "BP"))
    (Components|Movement|StopMovementImmediately (Variables|Default|GetProjectileMovement))))

(event OnComponentBeginOverlap(SphereCollision)
  (params (OtherActor :type Actor%20Object%20Reference) (OtherComp :type Primitive%20Component%20Object%20Reference) (OtherBodyIndex :type Integer) (bFromSweep :type Boolean) (SweepResult :type Hit%20Result%20Structure%20%28by%20ref%29))
  ;[0.00015 0.0113 1] HealthPickup
  (Utilities|FlowControl|Gate true
    (:Exit
      (switch string (Utilities|GetClassDisplayName (Utilities|GetClass OtherActor))
        (:William_C
          (Class|DamageInterface|CanTakeDamage(Message) OtherActor (Variables|Default|GetDamage) (Utilities|GetClassDisplayName (Utilities|GetClass self)) self)
          (Variables|Default|SetbAutoDestroyWhenFinished true))))))

(event OnComponentBeginOverlap(Sphere)
  (params (OtherActor :type Actor%20Object%20Reference) (OtherComp :type Primitive%20Component%20Object%20Reference) (OtherBodyIndex :type Integer) (bFromSweep :type Boolean) (SweepResult :type Hit%20Result%20Structure%20%28by%20ref%29))
  ;[1 0.8805 0] On begin overlap of the actual health droplet
  (Utilities|FlowControl|Gate true
    (:Exit
      (switch string (Utilities|GetClassDisplayName (Utilities|GetClass OtherActor))
        (:Default
          (Class|DamageInterface|CanTakeDamage(Message) OtherActor (Variables|Default|GetDamage) (Utilities|GetClassDisplayName (Utilities|GetClass self)) self)
          (Variables|Default|SetbAutoDestroyWhenFinished true))
        (:MakyaSplash_C
          (Actor|DestroyActor))))))

(event OnProjectileStop(ProjectileMovement)
  (params (ImpactResult :type Hit%20Result%20Structure%20%28by%20ref%29))
  ;[1 0.008681 0] Bounce off certain actors, stick to everything else
  (Components|Activation|Deactivate (Variables|Default|GetParticleSystem)))

(event Custom|OnOverlapGateOpen
  ;[0.00015 0.0113 1] HealthPickup
  (Utilities|FlowControl|Gate true) ; enters at Open
)

(event Custom|OnOverlapGateOpen1
  ;[1 0.8805 0] On begin overlap of the actual health droplet
  (Utilities|FlowControl|Gate true) ; enters at Open
)

(event EventBeginPlay
  ;[0 1 0.03525] Invuln Timer
  (Utilities|FlowControl|Delay 0.4)
  (CallFunction|OnOverlapGateOpen)
  (CallFunction|OnOverlapGateOpen1))

(event EventTick
  (params (DeltaSeconds :type Float%20%28single-precision%29))
  (bind _returnvalue (/ DeltaSeconds 155.0))
  (bind _sphere (Variables|Default|GetSphere))
  (bind _sphere_2 (Variables|Default|GetSphere))
  (bind _returnvalue_2 (Transformation|GetWorldScale _sphere_2))
  (bind _returnvalue_3 (Transformation|GetWorldScale _sphere))
  ;[1 0 0.8839] Get smaller over time
  (Transformation|SetWorldScale3D (Variables|Default|GetSphere) (Math|Vector|MakeVector (- (.x _returnvalue_3) _returnvalue) (- (.y _returnvalue_3) _returnvalue) (- (.z _returnvalue_3) _returnvalue)))
  (if (Math|Boolean|ORBoolean (< (.x _returnvalue_2) 0.0) (< (.y _returnvalue_2) 0.0) (< (.z _returnvalue_2) 0.0))
    (Variables|Default|SetbAutoDestroyWhenFinished true)))

(fn ConstructionScript
  (Variables|/Script/Engine.ProjectileMovementComponent|SetInitialSpeed (Variables|Default|GetProjectileMovement) (Variables|Default|GetInitSpeed)))