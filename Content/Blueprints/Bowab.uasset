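; Bowab is a rolling enemy character that becomes active when William enters its trigger sphere, then repeatedly charges at its Target.
; A looping BeginPlay graph turns it via RotatingMovement along the shorter yaw direction until it faces the Target.
; It then locks that heading while a timeline drives movement input and pitch spin for the roll, re-aiming when the timeline finishes.
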(event OnComponentBeginOverlap(Sphere)
  (params (OtherActor :type Actor%20Object%20Reference) (OtherComp :type Primitive%20Component%20Object%20Reference) (OtherBodyIndex :type Integer) (bFromSweep :type Boolean) (SweepResult :type Hit%20Result%20Structure%20%28by%20ref%29))
  ;[1 1 1] Anger the bowab
  (if (== (Utilities|GetClass OtherActor) "/Game/Blueprints/William.William_C")
    (Variables|Default|SetActive true)))

(event EventBeginPlay
  (bind _returnvalue (Transformation|GetActorLocation))
  (bind _returnvalue_2 (Transformation|GetActorRotation))
  (bind _returnvalue_3 (Transformation|GetWorldRotation))
  (bind _rotatingmovement (Variables|Default|GetRotatingMovement))
  (bind _target (Variables|Default|GetTarget))
  (bind _returnvalue_4 (Transformation|GetActorLocation _target))
  (bind _returnvalue_5 (Math|Rotator|FindLookatRotation _returnvalue _returnvalue_4))
  (bind _returnvalue_6 (- (.yaw _returnvalue_5) (.yaw _returnvalue_2)))
  ;[1 1 1] Infinite loop logic
  (if (Variables|Default|GetActive) :!label _label
    ;[1 1 1] Rotate towards player
    (if (or (and (> _returnvalue_6 -1.8e+02) (< _returnvalue_6 0.0)) (> _returnvalue_6 1.8e+02))
      (Variables|/Script/Engine.RotatingMovementComponent|SetRotationRate _rotatingmovement (Math|Rotator|MakeRotator 0.0 -6e+01 0.0))
      (else
        (Variables|/Script/Engine.RotatingMovementComponent|SetRotationRate _rotatingmovement (Math|Rotator|MakeRotator 0.0 6e+01 0.0))))
    (if (Math|Float|NearlyEqual(Float) (.yaw (Math|Rotator|FindLookatRotation (Transformation|GetActorLocation) (Transformation|GetActorLocation (Variables|Default|GetTarget)))) (.yaw (Transformation|GetActorRotation)) 2.0) :!label _label_2
      (Variables|/Script/Engine.RotatingMovementComponent|SetRotationRate (Variables|Default|GetRotatingMovement) "0, 0, 0")
      ;[1 1 1] Get the direction to move in
      (Variables|Default|SetFoward%20Vector (Math|Vector|GetForwardVector (Class|KismetMathLibrary|MakeRot 0.0 (.yaw _returnvalue_3) 0.0)))
      (Variables|Default|SetYaw (.yaw _returnvalue_3))
      ;[1 1 1] Roll 4 times
      (bind (_direction _foward_movement_scale _rotation_0_360) (Timeline|Timeline_0 PlayFromStart)
        (:Update
          (Pawn|Input|AddMovementInput (Variables|Default|GetFoward%20Vector) _foward_movement_scale false)
          (Transformation|SetActorRotation (Math|Rotator|MakeRotator _rotation_0_360 (Variables|Default|GetYaw) 0.0)))
        (:Finished
          (goto _label)))
      (else
        (Utilities|FlowControl|Delay 0.0)
        (goto _label_2)))
    (else
      (Utilities|FlowControl|Delay 0.2)
      (goto _label))))

(fn ConstructionScript)